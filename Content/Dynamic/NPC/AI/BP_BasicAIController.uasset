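; AI controller for NPC TP_Character pawns that runs BT_BasicAI on the BB_BasicAI blackboard.
; AI perception writes any sensed actor to the Enemy key, and on losing it stores LastSeenLocation and clears Enemy.
; Each tick, the pawn's Aiming and Shooting flags mirror whether the controller has a valid focus actor, which this graph never sets itself.
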(event OnTargetPerceptionUpdated(AIPerception)
  (params (Actor :type Actor%20Object%20Reference) (Stimulus :type AI%20Stimulus%20Structure))
  (bind (_age _expirationage _strength _stimuluslocation _receiverlocation _tag _bsuccessfullysensed) (Utilities|Struct|BreakAIStimulus Stimulus))
  (bind _returnvalue (Utilities|Name|MakeLiteralName "Enemy"))
  (bind _usingblackboard (Variables|Default|GetUsingBlackBoard))
  (if _bsuccessfullysensed
    (AI|Components|Blackboard|SetValueasObject _usingblackboard _returnvalue Actor)
    (else
      (AI|Components|Blackboard|SetValueasVector _usingblackboard (Utilities|Name|MakeLiteralName "LastSeenLocation") _stimuluslocation)
      (AI|Components|Blackboard|ClearValue _usingblackboard _returnvalue))))

(event EventBeginPlay
  (bind _blackboardcomponent (Class|AIController|UseBlackboard "/Game/Dynamic/NPC/AI/BB_BasicAI.BB_BasicAI"))
  (Variables|Default|SetUsingBlackBoard _blackboardcomponent)
  (AI|RunBehaviorTree "/Game/Dynamic/NPC/AI/BT_BasicAI.BT_BasicAI"))

(event EventTick
  (params (DeltaSeconds :type Float%20%28single-precision%29))
  (bind _returnvalue (Class|AIController|GetFocusActor))
  (bind _returnvalue_2 (Utilities|IsValid _returnvalue))
  (bind _astp_character (Utilities|Casting|CastToTP_Character (Pawn|GetControlledPawn)))
  (Variables|/Game/Dynamic/NPC/Behaviour/TP_Character.TP_Character_C|SetAiming? _astp_character _returnvalue_2)
  (Variables|/Game/Dynamic/NPC/Behaviour/TP_Character.TP_Character_C|SetShooting? _astp_character _returnvalue_2))

(fn ConstructionScript)