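; Terrain tile for an infinite terrain mode that scatters containers, sandbags, rocks, boxes and canisters on BeginPlay through PlaceActor.
; The player entering the Box trigger opens the green Wall barrier; leaving it closes the barrier in red and asks InfiniteTerrainGameMode to spawn another tile.
; The player entering Box2 calls CleanActors and destroys the tile.
; GetSnapPoint exposes the Arrow's world transform as an attachment point.
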(event OnComponentEndOverlap(Box)
  (params (OverlappedComponent :type Primitive%20Component%20Object%20Reference) (OtherActor :type Actor%20Object%20Reference) (OtherComp :type Primitive%20Component%20Object%20Reference) (OtherBodyIndex :type Integer))
  (Utilities|IsPlayer? OtherActor)
  (CallFunction|SetCollision)
  (bind _asinfinite_terrain_game_mode (Utilities|Casting|CastToInfiniteTerrainGameMode (Game|GetGameMode)))
  (Default|SpawnTile _asinfinite_terrain_game_mode))

(event OnComponentBeginOverlap(Box2)
  (params (OverlappedComponent :type Primitive%20Component%20Object%20Reference) (OtherActor :type Actor%20Object%20Reference) (OtherComp :type Primitive%20Component%20Object%20Reference) (OtherBodyIndex :type Integer) (bFromSweep :type Boolean) (SweepResult :type Hit%20Result%20Structure%20%28by%20ref%29))
  (Utilities|IsPlayer? OtherActor)
  (Class|Tile|CleanActors)
  (Actor|DestroyActor))

(event OnComponentBeginOverlap(Box)
  (params (OverlappedComponent :type Primitive%20Component%20Object%20Reference) (OtherActor :type Actor%20Object%20Reference) (OtherComp :type Primitive%20Component%20Object%20Reference) (OtherBodyIndex :type Integer) (bFromSweep :type Boolean) (SweepResult :type Hit%20Result%20Structure%20%28by%20ref%29))
  (Utilities|IsPlayer? OtherActor)
  (CallFunction|SetNoCollision))

(event EventBeginPlay
  (Class|Tile|PlaceActor "/Game/Dynamic/Terrain/Props/BP_Container.BP_Container_C" 2 3 3.6e+02 1.0 1.0)
  (Class|Tile|PlaceActor "/Game/Dynamic/Terrain/Props/BP_Sandbags.BP_Sandbags_C" 1 2 2e+02 1.0 1.0)
  (Class|Tile|PlaceActor "/Game/Dynamic/Terrain/Props/BP_Rock_01.BP_Rock_01_C" 1 2 1.5e+02 1.0 3.0)
  (Class|Tile|PlaceActor "/Game/Dynamic/Terrain/Props/BP_Rock_05.BP_Rock_05_C" 1 1 2e+02 1.0 4.0)
  (Class|Tile|PlaceActor "/Game/Dynamic/Terrain/Props/BP_Rock_17.BP_Rock_17_C" 1 2 2e+02 1.0 2.5)
  (Class|Tile|PlaceActor "/Game/Dynamic/Terrain/Props/BP_Box.BP_Box_C" 4 6 5e+01 1.0 1.0)
  (Class|Tile|PlaceActor "/Game/Dynamic/Terrain/Props/BP_Canister.BP_Canister_C" 4 6 25.0 1.0 1.0))

(event Collision|EventActorBeginOverlap
  (params (OtherActor :type Actor%20Object%20Reference)))

(event EventTick
  (params (DeltaSeconds :type Float%20%28single-precision%29)))

(fn ConstructionScript)

(fn GetSnapPoint
  (return (Transformation|GetWorldTransform (Variables|Default|GetArrow))))

(fn SetNoCollision
  (Collision|SetCollisionEnabled (Variables|Default|GetWall) "NoCollision")
  (Rendering|Material|SetMaterial (Variables|Default|GetWall) 0 "/Game/Dynamic/Terrain/M_BarrierGreen.M_BarrierGreen"))

(fn SetCollision
  (Collision|SetCollisionEnabled (Variables|Default|GetWall) "QueryAndPhysics")
  (Rendering|Material|SetMaterial (Variables|Default|GetWall) 0 "/Game/Dynamic/Terrain/M_BarrierRed.M_BarrierRed"))