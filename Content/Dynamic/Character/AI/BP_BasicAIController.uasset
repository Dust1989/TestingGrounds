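; BP_BasicAIController is an AI controller that feeds perception results into a basic behavior tree.
; On BeginPlay it sets up the BB_BasicAI blackboard and runs BT_BasicAI.
; Perception updates for actors without the "Enemy" tag set the blackboard's Enemy key when sensed and clear it when lost, printing a debug message either way.
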(event OnTargetPerceptionUpdated(AIPerception)
  (params (Actor :type Actor%20Object%20Reference) (Stimulus :type AI%20Stimulus%20Structure))
  (bind _returnvalue (Utilities|Name|MakeLiteralName "Enemy"))
  (bind _usingblackboard (Variables|Default|GetUsingBlackBoard))
  (if (not (Actor|ActorHasTag Actor "Enemy"))
    (if (.bSuccessfullySensed (Utilities|Struct|BreakAIStimulus Stimulus))
      (AI|Components|Blackboard|SetValueasObject _usingblackboard _returnvalue Actor)
      (Development|PrintString "Find")
      (else
        (AI|Components|Blackboard|ClearValue _usingblackboard _returnvalue)
        (Development|PrintString "Lost" true true "(R=0.112205,G=1.000000,B=0.000000,A=1.000000)")))))

(event EventBeginPlay
  (bind _blackboardcomponent (Class|AIController|UseBlackboard "/Game/Dynamic/Character/AI/BB_BasicAI.BB_BasicAI"))
  (Variables|Default|SetUsingBlackBoard _blackboardcomponent)
  (AI|RunBehaviorTree "/Game/Dynamic/Character/AI/BT_BasicAI.BT_BasicAI"))

(fn ConstructionScript)