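; Game mode for an infinite terrain level that spawns chained BP_Tile actors and tracks the score.
; On BeginPlay it fills a bounds volume pool, then spawns two tiles, with AI spawning enabled only on the second.
; SpawnTile places each tile at the stored snap point, hands it the shared NavMesh pool and stores its snap point for the next.
; SetScore increments the score by one.
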(event EventBeginPlay
  (Class|InfiniteTerrainGameMode|PopulateBoundsVolumePool)
  (for _index (range 0 1)
    (CallFunction|SpawnTile (> _index 0))))

(event EventTick
  (params (DeltaSeconds :type Float%20%28single-precision%29)))

(fn ConstructionScript)

(fn SpawnTile
  (params (SpawnAI :type Boolean))
  (bind _returnvalue (Game|SpawnActorfromClass "/Game/Dynamic/Terrain/BP_Tile.BP_Tile_C" (Variables|Default|GetNextSnapPoint) "Undefined" 0 SpawnAI 0))
  (Class|Tile|SetNavMeshPool _returnvalue (Variables|Default|GetNavMeshPool))
  (Variables|Default|SetNextSnapPoint (Default|GetSnapPoint _returnvalue)))

(fn GetScore
  (return (Variables|Default|GetScore)))

(fn SetScore
  (Variables|Default|SetScore (+ (Variables|Default|GetScore) 1)))